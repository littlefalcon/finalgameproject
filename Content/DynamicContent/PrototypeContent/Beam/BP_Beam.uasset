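; BP_Beam is a prototype beam effect for the first-person character's weapon.
; Each Tick it reads the player character's muzzle and hit locations and feeds them to its particle system as BeamSource and BeamTarget vector parameters.
; The beam shows only while the first weapon is selected and the left mouse button is held, polled directly from the player controller.
; It also prints the muzzle location every frame.
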(event `self.ReceiveTick`
  (params (DeltaSeconds :type "Float (single-precision)"))
  (bind _particlesystemcomponent (`self.ParticleSystemComponent`))
  (bind _particlesystemcomponent_2 (`self.ParticleSystemComponent`))
  (bind _asbp_first_person_character (cast `/Game/DynamicContent/PrototypeContent/BP_FirstPersonCharacter` (`GameplayStatics.GetPlayerCharacter` 0)))
  (bind _muzzlelocation (`SpaceHorrorCharacter.MuzzleLocation` _asbp_first_person_character))
  (`KismetSystemLibrary.PrintString` (`KismetStringLibrary.Conv_VectorToString` _muzzlelocation) true true (struct :`G` 0.66 :`B` 1.0 :`A` 1.0) 0.0001)
  (`ParticleSystemComponent.SetVectorParameter` _particlesystemcomponent_2 "BeamSource" _muzzlelocation)
  (`ParticleSystemComponent.SetVectorParameter` _particlesystemcomponent_2 "BeamTarget" (`/Game/DynamicContent/PrototypeContent/BP_FirstPersonCharacter.HitLocation` _asbp_first_person_character))
  (if (and (== (`SpaceHorrorCharacter.WeaponSelecter` _asbp_first_person_character) 0) (`PlayerController.IsInputKeyDown` (`GameplayStatics.GetPlayerController` 0) "LeftMouseButton"))
    (`SceneComponent.SetVisibility` _particlesystemcomponent true true)
    (else
      (`SceneComponent.SetVisibility` _particlesystemcomponent false true))))

(fn `UserConstructionScript`)